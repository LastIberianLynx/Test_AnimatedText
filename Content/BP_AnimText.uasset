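; BP_AnimText is a text actor that displays a configurable string and color through a TextRender component.
; On BeginPlay it applies both, then creates a dynamic instance of the text material and passes in fade-out speed, scale-down and move-up values.
; The Blueprint runs no Tick logic, so any animation from these parameters is left to the material.
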(event EventBeginPlay
  (bind _textrender (Variables|Default|GetTextRender))
  (Rendering|Components|TextRender|SetText _textrender (Variables|Default|GetText))
  (Rendering|Components|TextRender|SetTextRenderColor _textrender (Variables|Default|GetColor))
  (bind _returnvalue (Rendering|Material|CreateDynamicMaterialInstance (Variables|Default|GetTextRender) 0 (Rendering|Material|GetMaterial (Variables|Default|GetTextRender) 0) "None" :!class /Script/Engine.PrimitiveComponent))
  (Rendering|Material|SetScalarParameterValue _returnvalue "FadeOutSpeed" (Variables|Default|GetFadeOutSpeed) :!class /Script/Engine.MaterialInstanceDynamic)
  (Rendering|Material|SetScalarParameterValue _returnvalue "Scale" (Variables|Default|GetScaleDown) :!class /Script/Engine.MaterialInstanceDynamic)
  (Rendering|Material|SetScalarParameterValue _returnvalue "MoveUp" (Variables|Default|GetMoveUp) :!class /Script/Engine.MaterialInstanceDynamic))

(event EventTick
  (params (DeltaSeconds :type Float%20%28single-precision%29)))

(fn ConstructionScript)